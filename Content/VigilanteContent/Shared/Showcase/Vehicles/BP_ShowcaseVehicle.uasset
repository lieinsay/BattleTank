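; BP_ShowcaseVehicle is a vehicle showcase actor that exposes its display data through getter functions.
; It holds an array of showcase cameras, readable by index or count, along with a name and a slot.
; It has no active event or construction logic, so any camera switching or presentation is not handled in its graphs.
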(fn `GetShowcaseCamera`
  (params (Index :type Integer))
  (returns (Camera :type "CameraActor Object Reference"))
  (return (`|GetArrayItem` (`self.ShowcaseCameras`) Index)))

(fn `GetShowcaseCameraCount`
  (returns (Count :type Integer))
  (return (`KismetArrayLibrary.Array_Length` (`self.ShowcaseCameras`))))

(fn `GetShowcaseName`
  (returns (Name :type String))
  (return (`self.Name`)))

(fn `GetShowcaseSlot`
  (returns (Slot :type Integer))
  (return (`self.Slot`)))

(fn `UserConstructionScript`)