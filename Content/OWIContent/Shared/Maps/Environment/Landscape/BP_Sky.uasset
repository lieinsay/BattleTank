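; Sky dome actor that renders a textured sky with a sun disc through a dynamic instance of M_env_sky.
; The construction script pins the mesh to the world origin and sets texture and sun parameters, with RefreshMaterial as a details-panel rerun toggle.
; Sun direction follows an assigned directional light, otherwise SunHeight and actor yaw, and negative height blends in stars.
; UpdateSunDirection re-applies the light-driven sun parameters without checking the light is valid.
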(fn `UpdateSunDirection`
  (bind _sky_material_dim (`self.Sky material DIM`))
  (bind _sun_height (`self.Sun Height`))
  (`MaterialInstanceDynamic.SetVectorParameterValue` _sky_material_dim "Light direction" (`KismetMathLibrary.Conv_VectorToLinearColor` (`KismetMathLibrary.Conv_RotatorToVector` (`self.K2_GetActorRotation` (`self.Directional light actor`)))))
  (`MaterialInstanceDynamic.SetVectorParameterValue` _sky_material_dim "Sun color" (* (`self.Sun Color`) (`self.Sun Brightness`)))
  (set `self.Sun Height` (`KismetMathLibrary.MapRangeUnclamped` (.pitch (`self.K2_GetActorRotation` (`self.Directional light actor`))) 0.0 -90.0 0.0 1.0))
  (`MaterialInstanceDynamic.SetScalarParameterValue` (`self.Sky material DIM`) "Sun height" (`KismetMathLibrary.SelectFloat` (`KismetMathLibrary.Abs` _sun_height) 0.0 (< _sun_height 0.0)))
  (`MaterialInstanceDynamic.SetScalarParameterValue` (`self.Sky material DIM`) "Sun Radius" (`self.Sun Radius`)))

(fn `UserConstructionScript`
  (bind _sky_material_dim (`self.Sky material DIM`))
  (bind _sky_material_dim_2 (`self.Sky material DIM`))
  (bind _sky_material_dim_3 (`self.Sky material DIM`))
  (bind _sun_height (`self.Sun Height`))
  (bind _sky_material_dim_4 (`self.Sky material DIM`))
  (`SceneComponent.K2_SetWorldLocation` (`self.Sky Sphere mesh`) (0.0 0.0 0.0) false false)
  (bind _returnvalue (`PrimitiveComponent.CreateDynamicMaterialInstance` (`self.Sky Sphere mesh`) 0 "/Game/OWIContent/Shared/Maps/Environment/Landscape/Textures/M_env_sky.M_env_sky" "None"))
  (bind _output_get (set `self.Sky material DIM` _returnvalue))
  (`MaterialInstanceDynamic.SetTextureParameterValue` _output_get "SkyTexture" (`self.Sky Texture`))
  ;[1 1 1] Skybox Texture Params
  (`MaterialInstanceDynamic.SetVectorParameterValue` _sky_material_dim "ST_Dome Position Offset" (`KismetMathLibrary.Conv_VectorToLinearColor` (`self.Dome Position Offset`)))
  (`MaterialInstanceDynamic.SetVectorParameterValue` _sky_material_dim "ST_Camera Vector Multiplier" (`KismetMathLibrary.Conv_VectorToLinearColor` (`self.ST_Camera Vector Multiplier`)))
  (`MaterialInstanceDynamic.SetScalarParameterValue` _sky_material_dim "ST_Dome Rotation  Z" (`self.ST_Dome Rotation  Z`))
  (`MaterialInstanceDynamic.SetScalarParameterValue` _sky_material_dim "ST_Dome V scale" (select `bool` (`self.Hemisphere`) :`false` 1.0 :`true` 2.0 :!type "Float (single-precision)"))
  (`MaterialInstanceDynamic.SetScalarParameterValue` _sky_material_dim_4 "ST_Brightness" (`self.Brigntness`))
  (`MaterialInstanceDynamic.SetScalarParameterValue` _sky_material_dim_4 "ST_Contrast" (`self.Contrast`))
  (`MaterialInstanceDynamic.SetScalarParameterValue` _sky_material_dim_4 "ST_Desaturation" (`self.Desaturation`))
  (if (`self.Refresh material`)
    _
    (else
      _))
  ;[1 1 1] Set Sun Disc Params
  (set `self.Refresh material` false)
  (`/Engine/EditorBlueprintResources/StandardMacros.IsValid` (`self.Directional light actor`) ; Has a directional light been assigned?
    (:`Is Valid`
      (`MaterialInstanceDynamic.SetVectorParameterValue` _sky_material_dim_2 "Light direction" (`KismetMathLibrary.Conv_VectorToLinearColor` (`KismetMathLibrary.Conv_RotatorToVector` (`self.K2_GetActorRotation` (`self.Directional light actor`)))))
      (`MaterialInstanceDynamic.SetVectorParameterValue` _sky_material_dim_2 "Sun color" (* (`self.Sun Color`) (`self.Sun Brightness`)))
      (set `self.Sun Height` (`KismetMathLibrary.MapRangeUnclamped` (.pitch (`self.K2_GetActorRotation` (`self.Directional light actor`))) 0.0 -90.0 0.0 1.0)))
    (:`Is Not Valid`
      (`MaterialInstanceDynamic.SetVectorParameterValue` _sky_material_dim_3 "Light direction" (`KismetMathLibrary.Conv_VectorToLinearColor` (`KismetMathLibrary.Conv_RotatorToVector` (`KismetMathLibrary.MakeRotator` 0.0 (`KismetMathLibrary.MapRangeUnclamped` (`self.Sun Height`) -1.0 1.0 90.0 -90.0) (.yaw (`self.K2_GetActorRotation`))))))
      (`MaterialInstanceDynamic.SetVectorParameterValue` _sky_material_dim_3 "Sun color" (`KismetMathLibrary.LinearColorLerp` (struct :`R` 1.0 :`G` 0.221 :`B` 0.04 :`A` 1.0) (struct :`R` 0.954 :`G` 0.901 :`B` 0.74412 :`A` 1.0) (`KismetMathLibrary.FClamp` (+ (`self.Sun Height`) 0.2))))))
  (`MaterialInstanceDynamic.SetScalarParameterValue` (`self.Sky material DIM`) "Sun brightness" (`self.Sun Brightness`))
  (`MaterialInstanceDynamic.SetScalarParameterValue` (`self.Sky material DIM`) "Sun height" (`KismetMathLibrary.SelectFloat` (`KismetMathLibrary.Abs` _sun_height) 0.0 (< _sun_height 0.0)))
  (`MaterialInstanceDynamic.SetScalarParameterValue` (`self.Sky material DIM`) "Sun Radius" (`self.Sun Radius`)))